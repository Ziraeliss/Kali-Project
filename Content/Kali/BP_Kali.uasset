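; BP_Kali is the player's sword companion actor, registering itself as SwordActor on PC_Default at BeginPlay.
; Each Tick it eases toward a point behind the player, except while the player glides or skates.
; A non-zero target from SetAimingPosition disables its skate and glide components and snaps it there, since GetAimingAlpha always returns 1.
; While that target is set, aim mode being off clears it and re-enables both.
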(event `self.ReceiveBeginPlay`
  (bind _aspc_default (cast `/Game/ThirdPerson/Blueprints/PC_Default` (`GameplayStatics.GetPlayerController` 0)))
  (set `/Game/ThirdPerson/Blueprints/PC_Default.SwordActor` self _aspc_default))

(event `self.ReceiveTick`
  (params (DeltaSeconds :type "Float (single-precision)"))
  (bind _returnvalue (`GameplayStatics.GetPlayerPawn` 0))
  (bind _returnvalue_2 (`GameplayStatics.GetPlayerCharacter` 0))
  (bind _ac_glidecomponent (`self.AC_GlideComponent`))
  (bind _ac_skatecomponent (`self.AC_SkateComponent`))
  (bind _valid (`self.TargetPositionValid`))
  (if _valid
    (set `/Game/ThirdPerson/Blueprints/AC_SkateComponent.CanSkate` false _ac_skatecomponent)
    (set `/Game/ThirdPerson/Blueprints/AC_GlideComponent.ShouldGlide` false _ac_glidecomponent)
    (`self.K2_SetActorLocation` (`KismetMathLibrary.VLerp` (`self.InitialPosition`) (`self.TargetPosition`) (`self.GetAimingAlpha`)))
    (bind _asbp_third_person_character (cast `/Game/ThirdPerson/Blueprints/BP_ThirdPersonCharacter` _returnvalue_2))
    (if (not (`/Game/ThirdPerson/Blueprints/BP_ThirdPersonCharacter.AimingModeOn` _asbp_third_person_character))
      (set `self.TargetPosition` (0.0 0.0 0.0))
      (set `/Game/ThirdPerson/Blueprints/AC_SkateComponent.CanSkate` true _ac_skatecomponent)
      (set `/Game/ThirdPerson/Blueprints/AC_GlideComponent.ShouldGlide` true _ac_glidecomponent))
    (else
      (set `/Game/ThirdPerson/Blueprints/AC_SkateComponent.CanSkate` true _ac_skatecomponent)
      (set `/Game/ThirdPerson/Blueprints/AC_GlideComponent.ShouldGlide` true _ac_glidecomponent)
      (bind _asbp_third_person_character_2 (cast `/Game/ThirdPerson/Blueprints/BP_ThirdPersonCharacter` _returnvalue_2))
      (if (`/Game/ThirdPerson/Blueprints/BP_ThirdPersonCharacter.IsGliding` _asbp_third_person_character_2)
        _
        (elif (not (`/Game/ThirdPerson/Blueprints/BP_ThirdPersonCharacter.IsSkating` _asbp_third_person_character_2))
          (`self.K2_SetActorLocation` (`KismetMathLibrary.VInterpTo` (`self.K2_GetActorLocation`) (+ (`self.K2_GetActorLocation` _returnvalue) (* (`self.GetActorForwardVector` _returnvalue) -150.0)) DeltaSeconds 10.0)))))))

(fn `GetAimingAlpha`
  (returns (NewAlpha :type "Float (double-precision)"))
  (return 1.0))

(fn `SetAimingPosition`
  (params (NewPosition :type "Vector Structure") (NewRotation :type "Rotator Structure"))
  (set `self.TargetPosition` NewPosition)
  (set `self.TargetRotation` NewRotation)
  (set `self.InitialPosition` (`self.K2_GetActorLocation`)))

(fn `SetCollisionType`
  (params (CollisionType :type "ECollisionEnabled Enum" :default "NoCollision"))
  (`PrimitiveComponent.SetCollisionEnabled` (`self.BoxCollider`) CollisionType))

(fn `TargetPositionValid`
  (returns (Valid :type Boolean))
  (return (!= (`self.TargetPosition`) (0.0 0.0 0.0))))

(fn `UserConstructionScript`)